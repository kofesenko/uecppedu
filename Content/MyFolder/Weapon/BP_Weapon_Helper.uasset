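; BP_Weapon_Helper is a weapon Blueprint that handles firing, clip and reserve ammo, and timed reloading.
; FIre checks CanFire, runs a debug-drawn box trace from the muzzle socket without using the hit, then spends ammo and auto-reloads on empty.
; Reload sets a timer to Finish Reload, which sets, rather than adds to, the clip count using the amount taken from reserve.
; Print strings report ammo and reload state.
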(event EventReload
  (bind _result (CallFunction|CanReload))
  (if _result
    (Variables|Default|SetbIsReloading true)
    (Development|PrintString "Start Reload")
    (Utilities|Time|SetTimerbyFunctionName 0 "Finish Reload" (Variables|Configs|GetReloadDuration))))

(fn ConstructionScript)

(fn WeaponTrace
  (bind _muzzlesocketname (Variables|Configs|GetMuzzleSocketName))
  (bind _mesh (Variables|Default|GetMesh))
  (bind _returnvalue (Transformation|GetSocketLocation _mesh _muzzlesocketname))
  (Class|KismetSystemLibrary|BoxTraceSinglebyProfile _returnvalue (+ _returnvalue (* (Math|Vector|GetForwardVector (Variables|Default|GetMesh)) (Variables|Configs|GetRange))) "0, 0, 0" "0, 0, 0" "None" false 0 "ForDuration" true "(R=1.000000,G=0.000000,B=0.000000,A=1.000000)" "(R=0.000000,G=1.000000,B=0.000000,A=1.000000)" 0.5))

(fn FIre
  (if (CallFunction|CanFire)
    (CallFunction|WeaponTrace)
    (CallFunction|UseAmmo)))

(fn UseAmmo
  (bind _result (Math|Integer|DecrementInt (Variables|Default|GetCurrentAmmoInClip))
    (:%20%20
      (Development|PrintString (Utilities|String|ToString(Integer) _result))
      (bind _result_2 (CallFunction|CanReload))
      (if (and _result_2 (<= (Variables|Default|GetCurrentAmmoInClip) 0))
        (CallFunction|Reload)))))

(fn CanFire
  (return (and (> (Variables|Default|GetCurrentAmmoInClip) 0) (not (Variables|Default|GetbIsReloading)))))

(fn FinishReload
  (LocalVariables|SetAmmoForReload (CallFunction|GetAmmoforReload))
  (Variables|Default|SetCurrentAmmoInClip (LocalVariables|GetAmmoForReload))
  (Variables|Default|SetCurrentAmmo (- (Variables|Default|GetCurrentAmmo) (LocalVariables|GetAmmoForReload)))
  (Variables|Default|SetbIsReloading false)
  (Development|PrintString (Utilities|String|Append "Reloaded  " (Utilities|String|ToString(Integer) (Variables|Default|GetCurrentAmmoInClip)) " / " (Utilities|String|ToString(Integer) (Variables|Default|GetCurrentAmmo)))))

(fn GetAmmoforReload
  (LocalVariables|SetAmmoNeeded (- (Variables|Default|GetMaxAmmoInClip) (Variables|Default|GetCurrentAmmoInClip)))
  (if (>= (Variables|Default|GetCurrentAmmo) (LocalVariables|GetAmmoNeeded))
    (return (LocalVariables|GetAmmoNeeded))
    (else
      (return (Variables|Default|GetCurrentAmmo)))))

(fn CanReload
  (return (Math|Boolean|ANDBoolean (> (Variables|Default|GetMaxAmmoInClip) (Variables|Default|GetCurrentAmmoInClip)) (> (Variables|Default|GetCurrentAmmo) 0) (not (Variables|Default|GetbIsReloading)))))